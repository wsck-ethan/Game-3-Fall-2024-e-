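; BP_decoy is an AI decoy pawn that spawns with a fire actor on its mesh and runs forward.
; An enemy entering its sphere starts a delayed self-destruct and redirects it to that enemy, while melee-hit overlap plays a punch animation.
; A failed forward move also destroys decoy and fire after a delay.
; Pawn sensing only stores the seen pawn, and the looping bullet-attack event is not called here.
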(event `self.PawnSensing.OnSeePawn`
  (params (Pawn :type "Pawn Object Reference"))
  (set `self.enemy` Pawn)
  (set `self.enemylocation` (`self.K2_GetActorLocation` Pawn)))

(event `self.ReceiveBeginPlay`
  (bind _returnvalue (`|SpawnActorFromClass` "/Game/Yasagorgons/Ethan/ai/BP_fire_e.BP_fire_e_C" (`SceneComponent.K2_GetComponentToWorld` (`self.Arrow1`)) "Undefined" "MultiplyWithRoot" null null))
  (bind _output_get (set `self.fire` _returnvalue))
  (`SceneComponent.K2_AttachToComponent` (`Actor.RootComponent` _output_get) (`self.Mesh`) "fire" "SnapToTarget" "SnapToTarget" "SnapToTarget" true)
  (`|AIMoveTo` self (+ (* (`KismetMathLibrary.GetForwardVector` (`self.K2_GetActorRotation`)) 1500.0) (`self.K2_GetActorLocation`)) null
    (:`OnFail`
      (`KismetSystemLibrary.Delay` 5.0)
      (`self.K2_DestroyActor` (`self.fire`))
      (`self.K2_DestroyActor` self))))

(event `self.Sphere.OnComponentBeginOverlap`
  (params (OverlappedComponent :type "PrimitiveComponent Object Reference") (OtherActor :type "Actor Object Reference") (OtherComp :type "PrimitiveComponent Object Reference") (OtherBodyIndex :type Integer) (bFromSweep :type Boolean) (SweepResult :type "HitResult Structure (by ref)"))
  (bind _asbp_enemy_base (cast `/Game/AI_Blueprints/BP_Enemy_Base` OtherActor))
  (`self.desory self`)
  (`|AIMoveTo` self (0.0 0.0 0.0) _asbp_enemy_base))

(event `attackbullet`
  (`|SpawnActorFromClass` "/Game/Yasagorgons/Ethan/ai/BP_bullet.BP_bullet_C" (`KismetMathLibrary.MakeTransform` (`self.K2_GetActorLocation`) (`self.K2_GetActorRotation`)) "Undefined" "MultiplyWithRoot" null null :!label _label)
  (`KismetSystemLibrary.Delay` 0.2)
  (goto _label))

(event `desory self`
  (`KismetSystemLibrary.Delay` 5.0)
  (`self.K2_DestroyActor` self)
  (`self.K2_DestroyActor` (`self.fire`)))

(event `meleeAttack`
  (`SkeletalMeshComponent.PlayAnimation` (`self.Mesh`) "/Game/Yasagorgons/Ethan/anim/Punching__1_.Punching__1_" false))

(event `self.meleeHit.OnComponentBeginOverlap`
  (params (OverlappedComponent :type "PrimitiveComponent Object Reference") (OtherActor :type "Actor Object Reference") (OtherComp :type "PrimitiveComponent Object Reference") (OtherBodyIndex :type Integer) (bFromSweep :type Boolean) (SweepResult :type "HitResult Structure (by ref)"))
  (cast `/Game/AI_Blueprints/BP_Enemy_Base` OtherActor)
  (`self.meleeAttack`))

(fn `UserConstructionScript`)