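; Pickup skill that attaches to the player's left hand on overlap if no skill is held, then summons a moving decoy.
; BeginSkill, gated by cooldown, traces from the first-person camera, spawns a temporary fire effect and BP_decoy in front of it.
; AIMoveTo sends the decoy toward the trace hit, and mana is deducted as the move is issued.
; EndSkill calls StopSkill, starting a cooldown that recursively counts down through delays.
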(event `/Game/Blueprints/I_Skill.BeginSkill`
  (bind _as_bp_third_person_character (`self.As BP Third Person Character`))
  (bind _firstpersoncamera (`/Game/ThirdPerson/Blueprints/BP_ThirdPersonCharacter.FirstPersonCamera` _as_bp_third_person_character))
  (bind _firstpersoncamera_2 (`/Game/ThirdPerson/Blueprints/BP_ThirdPersonCharacter.FirstPersonCamera` (`self.As BP Third Person Character`)))
  (bind _returnvalue (`SceneComponent.K2_GetComponentLocation` _firstpersoncamera_2))
  (bind _returnvalue_2 (`SceneComponent.K2_GetComponentRotation` _firstpersoncamera_2))
  (`KismetSystemLibrary.PrintString` "spawning ")
  (if (<= (`self.Skill Cooldown`) 0.0)
    (set `self.Skill is Active` true)
    (bind _outhit (`KismetSystemLibrary.LineTraceSingle` :`Start` _returnvalue :`End` (+ _returnvalue (* (`KismetMathLibrary.GetForwardVector` _returnvalue_2) 1500.0)) :`TraceChannel` "TraceTypeQuery1" :`DrawDebugType` "ForDuration"))
    (bind _output_get (set `self.Location` (`.Location` (`GameplayStatics.BreakHitResult` _outhit))))
    (bind _output_get_2 (set `self.spawn location` (+ (`SceneComponent.K2_GetComponentLocation` _firstpersoncamera) (* (`KismetMathLibrary.GetForwardVector` (`SceneComponent.K2_GetComponentRotation` _firstpersoncamera)) 150.0))))
    (bind _returnvalue_3 (`|SpawnActorFromClass` "/Game/Yasagorgons/Ethan/ai/BP_fire_big.BP_fire_big_C" (`KismetMathLibrary.MakeTransform` _output_get_2) "Undefined" "MultiplyWithRoot" null null))
    (`KismetSystemLibrary.Delay` 1.0)
    (bind _returnvalue_4 (`|SpawnActorFromClass` "/Game/Yasagorgons/Ethan/ai/BP_decoy.BP_decoy_C" (`KismetMathLibrary.MakeTransform` _output_get_2 _returnvalue_2) "Undefined" "MultiplyWithRoot" null null))
    (`KismetSystemLibrary.Delay` 0.5)
    (`self.K2_DestroyActor` _returnvalue_3)
    (`|AIMoveTo` _returnvalue_4 _output_get null
      (:`then`
        (`/Game/ThirdPerson/Blueprints/BP_ThirdPersonCharacter.Update Player Stats` _as_bp_third_person_character 0.0 -0.4 0.0)))))

(event `Update Skill Cooldown`
  ;[1 1 1] As long as Cooldown is above zero, let's reduce that number and stop the player from starting up this skill again.
  (if (> (`self.Skill Cooldown`) 0.0)
    (bind _output_get (set `self.Skill Cooldown` (- (`self.Skill Cooldown`) 0.1)))
    (`KismetSystemLibrary.Delay` 0.1)
    (`KismetSystemLibrary.PrintString` (`KismetStringLibrary.Concat_StrStr` " cooldown is" (`KismetStringLibrary.Conv_DoubleToString` _output_get)) true true (struct :`G` 0.66 :`B` 1.0 :`A` 1.0) 0.1)
    (`self.Update Skill Cooldown`)))

(event `Stop Skill`
  (if (`self.Skill is Active`)
    (set `self.Skill is Active` false)
    (set `self.Skill Cooldown` 5.0) ; subtract whatever time the \nplayer still had for this effect
    (`self.Update Skill Cooldown`)
    (else
      (`KismetSystemLibrary.PrintString` "skill is already inactive"))))

(event `self.sphere collision.OnComponentBeginOverlap`
  (params (OverlappedComponent :type "PrimitiveComponent Object Reference") (OtherActor :type "Actor Object Reference") (OtherComp :type "PrimitiveComponent Object Reference") (OtherBodyIndex :type Integer) (bFromSweep :type Boolean) (SweepResult :type "HitResult Structure (by ref)"))
  (bind _asbp_third_person_character (cast `/Game/ThirdPerson/Blueprints/BP_ThirdPersonCharacter` OtherActor))
  (bind _output_get (set `self.As BP Third Person Character` _asbp_third_person_character))
  (`/Game/ThirdPerson/Blueprints/BP_ThirdPersonCharacter.CurrentSKill` _output_get
    (:`then`
      (`KismetSystemLibrary.PrintString` "You have  a skill!"))
    (:`else`
      (set `/Game/ThirdPerson/Blueprints/BP_ThirdPersonCharacter.CurrentSKill` self _output_get)
      (`self.K2_AttachToComponent` (`Character.Mesh` _output_get) "lhand" "SnapToTarget" "SnapToTarget" "SnapToTarget") ; attach this skill to the player's left hand
      (`KismetSystemLibrary.PrintString` "Holding SpawningSkill now!")
      (`ActorComponent.K2_DestroyComponent` (`self.Sphere1`)))))

(event `/Game/Blueprints/I_Skill.EndSkill`
  (`KismetSystemLibrary.PrintString` "Early End to BF Skill")
  (`self.Stop Skill`))

(fn `UserConstructionScript`)